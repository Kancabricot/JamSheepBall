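; Trigger actor that tilts the game camera when a BP_ScalableEnemy enters its TriggerForCamera component.
; On overlap it finds the BP_Camera in the level and captures the MainCamera's current world rotation.
; A timeline then lerps that rotation to a 45-degree negative roll offset, keeping pitch and yaw, with no logic to restore it.
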(event `self.TriggerForCamera.OnComponentBeginOverlap`
  (params (OverlappedComponent :type "PrimitiveComponent Object Reference") (OtherActor :type "Actor Object Reference") (OtherComp :type "PrimitiveComponent Object Reference") (OtherBodyIndex :type Integer) (bFromSweep :type Boolean) (SweepResult :type "HitResult Structure (by ref)"))
  (bind (_initialrot_roll _initialrot_pitch _initialrot_yaw) (`KismetMathLibrary.BreakRotator` (`self.InitialRot`)))
  (cast `/Game/Blueprints/ScalablObject/BP_ScalableEnemy` OtherActor)
  (bind _returnvalue (`GameplayStatics.GetActorOfClass` "/Game/Blueprints/Player/BP_Camera.BP_Camera_C"))
  (bind _maincamera (`/Game/Blueprints/Player/BP_Camera.MainCamera` _returnvalue))
  (set `self.InitialRot` (`SceneComponent.K2_GetComponentRotation` _maincamera))
  (bind (_direction _newtrack_0) (`Timeline|Timeline Rotation`)
    (:`Update`
      (`SceneComponent.K2_SetWorldRotation` _maincamera (`KismetMathLibrary.RLerp` (`self.InitialRot`) (`KismetMathLibrary.MakeRotator` (+ _initialrot_roll -45.0) _initialrot_pitch _initialrot_yaw) _newtrack_0) false false))))

(fn `UserConstructionScript`)