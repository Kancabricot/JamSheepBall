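; BP_WolfStart is a one-shot event actor that launches a referenced wolf along a spline when the player enters its trigger.
; After a short delay, the LauncheEnemy timeline curve drives the wolf's location along SplineLauncher, without sweeping.
; When the timeline finishes, it enables physics on the wolf's ScableObject and destroys WallToDestroy shortly afterwards.
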(event `self.TrigerForStart.OnComponentBeginOverlap`
  (params (OverlappedComponent :type "PrimitiveComponent Object Reference") (OtherActor :type "Actor Object Reference") (OtherComp :type "PrimitiveComponent Object Reference") (OtherBodyIndex :type Integer) (bFromSweep :type Boolean) (SweepResult :type "HitResult Structure (by ref)"))
  (if (`self.b_Init`)
    (cast `/Game/Blueprints/ScalablObject/BP_ScablePlayer` OtherActor)
    (set `self.b_Init` false)
    (`KismetSystemLibrary.Delay` 2.0)
    (bind (_direction _launchcrve) (`Timeline|LauncheEnemy` :!via `PlayFromStart`)
      (:`Update`
        (`self.K2_SetActorLocation` (`self.WolfRef`) (`SplineComponent.GetLocationAtDistanceAlongSpline` (`self.SplineLauncher`) (`KismetMathLibrary.Lerp` 0.0 (`SplineComponent.GetSplineLength` (`self.SplineLauncher`)) _launchcrve) "World") false false))
      (:`Finished`
        (`PrimitiveComponent.SetSimulatePhysics` (`/Game/Blueprints/ScalablObject/BP_ScalableParent.ScableObject` (`self.WolfRef`)) true)
        (`KismetSystemLibrary.Delay` 0.18)
        (`self.K2_DestroyActor` (`self.WallToDestroy`))))))

(fn `UserConstructionScript`)