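; Parent Blueprint for scalable objects, whose mesh is set at construction and can be scaled up or down, then eased back to its starting size.
; ScaleObject multiplies or divides the BeginPlay scale, per BScaleUp, when the multiplied size lies between the base and maximum multiple.
; After a delay, StartResizeToBaseScale runs a timeline that lerps back to the initial scale.
; StopResizeToBaseScale reverses that timeline.
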(event `self.ReceiveBeginPlay`
  (set `self.InitialScale` (`SceneComponent.K2_GetComponentScale` (`self.ScableObject`))))

(event `StartResizeToBaseScale`
  (`KismetSystemLibrary.K2_SetTimer` null "Start" 2.0))

(event `Start`
  (set `self.TempScale` (`SceneComponent.K2_GetComponentScale` (`self.ScableObject`)))
  (bind (_direction _resize) (`Timeline|ResizeToBaseScale` :!via `PlayFromStart` :!label _label)
    (:`Update`
      (`SceneComponent.SetWorldScale3D` (`self.ScableObject`) (`KismetMathLibrary.VLerp` (`self.TempScale`) (`self.InitialScale`) _resize)))))

(event `StopResizeToBaseScale`
  (goto _label :!via `Reverse`))

(fn `Scale Object`
  (params (ScaleMutiplier :type "Float (single-precision)"))
  (locals (b_IsUpScale :type Boolean))
  (bind _initialscale (`self.InitialScale`))
  (bind _returnvalue (* _initialscale ScaleMutiplier))
  (bind _returnvalue_2 (`KismetMathLibrary.VSize` _returnvalue))
  (bind _returnvalue_3 (and (<= _returnvalue_2 (`KismetMathLibrary.VSize` (* _initialscale (`self.MaxScaleMutiple`)))) (>= _returnvalue_2 (`KismetMathLibrary.VSize` _initialscale))))
  (if (`self.b_ScaleUp`)
    (if _returnvalue_3
      (`SceneComponent.SetWorldScale3D` (`self.ScableObject`) _returnvalue))
    (elif _returnvalue_3
      (`SceneComponent.SetWorldScale3D` (`self.ScableObject`) (/ _initialscale ScaleMutiplier)))))

(fn `UserConstructionScript`
  (`StaticMeshComponent.SetStaticMesh` (`self.ScableObject`) (`self.StaticMeshTarget`)))