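; BP_Camera is a camera actor that takes over the player's view and follows the player vertically.
; On BeginPlay, it becomes player controller 0's view target and starts a 0.001-second looping timer instead of using Tick.
; The timer interpolates its Z toward PlayerRef's CameraAttach component, keeping X and Y fixed.
; Following is skipped while BInTest is set or PlayerRef is invalid.
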(event `self.ReceiveBeginPlay`
  (`self.SetUp`))

(fn `SetCameraPos`
  (bind (_returnvalue_x _returnvalue_y _returnvalue_z) (`KismetMathLibrary.BreakVector` (`self.K2_GetActorLocation`)))
  (bind _playerref (`self.PlayerRef`))
  (bind (_returnvalue_x_2 _returnvalue_y_2 _returnvalue_z_2) (`KismetMathLibrary.BreakVector` (`SceneComponent.K2_GetComponentLocation` (`/Game/Blueprints/ScalablObject/BP_ScablePlayer.CameraAttach` _playerref))))
  (if (not (`self.b_InTest`))
    (`/Engine/EditorBlueprintResources/StandardMacros.IsValid` _playerref
      (:`Is Valid`
        (`self.K2_SetActorLocation` (`KismetMathLibrary.MakeVector` _returnvalue_x _returnvalue_y (`KismetMathLibrary.FInterpTo` _returnvalue_z _returnvalue_z_2 (`GameplayStatics.GetWorldDeltaSeconds`) (`self.Interp Speed`))))))))

(fn `SetUp`
  (`PlayerController.SetViewTargetWithBlend` (`GameplayStatics.GetPlayerController` 0) self 0.0 "VTBlend_Linear" 0.0 false)
  (`KismetSystemLibrary.K2_SetTimer` null "SetCameraPos" 0.001 true))

(fn `UserConstructionScript`)