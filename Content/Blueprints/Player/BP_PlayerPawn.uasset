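; Player pawn that lets the player click and drag with the mouse to scale BP_ScalableParent objects.
; On click start, a sphere trace under the cursor picks the target, anchors the camera's ImpactPoint, shows WG_UIScale and eases into slow motion via a timeline.
; While held, cursor distance from that anchor in the YZ plane drives the target's scale and UI length.
; Release or StopScaling removes the widget and reverses the time dilation.
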(event `self.ReceiveBeginPlay`
  (bind _returnvalue (`GameplayStatics.GetPlayerController` 0))
  ;[1 0.989 0] Setup Mouse and mapping
  (set `PlayerController.bShowMouseCursor` true _returnvalue)
  (`EnhancedInputSubsystemInterface.AddMappingContext` (pcsubsystem `EnhancedInputLocalPlayerSubsystem` _returnvalue) "/Game/Input/IMC_PLayerInput.IMC_PLayerInput" 0 (struct))
  (`WidgetBlueprintLibrary.SetInputMode_GameAndUIEx` (`GameplayStatics.GetPlayerController` 0) null "LockAlways" false)
  ;[0.3177 0.3177 0.3177] Get camera
  (bind _returnvalue_2 (`GameplayStatics.GetActorOfClass` "/Game/Blueprints/Player/BP_Camera.BP_Camera_C"))
  (set `self.CameraRef` _returnvalue_2))

(event `EnhancedInput|/Game/Input/InputAction/AI_Click`
  (params (ActionValue :type Boolean) (ElapsedSeconds :type "Float (double-precision)") (TriggeredSeconds :type "Float (double-precision)") (InputAction :type "InputAction Object Reference" :default "/Game/Input/InputAction/AI_Click.AI_Click"))
  (bind (_worldlocation _worlddirection) (`PlayerController.DeprojectMousePositionToWorld` (`GameplayStatics.GetPlayerController` 0)))
  ;[1 0 0] Scale system
  (:`Triggered`
    (if (`self.b_HaveTarget`)
      (`self.CalculateScale`)))
  (:`Started`
    ;;[1 1 1] Raycast with mouse
    (if (not (`self.b_IsEnd`))
      (bind _outhit (`KismetSystemLibrary.SphereTraceSingle` _worldlocation (+ _worldlocation (* _worlddirection 5000)) 10.0 "TraceTypeQuery1"))
      ;;[1 1 1] Check if we have valid target
      (bind _asbp_scalable_parent (cast `/Game/Blueprints/ScalablObject/BP_ScalableParent` (`.HitActor` (`GameplayStatics.BreakHitResult` _outhit)))
        (:`then`
          (set `self.TargetRef` _asbp_scalable_parent)
          (set `self.b_HaveTarget` true)
          (`SceneComponent.K2_SetWorldLocation` (`/Game/Blueprints/Player/BP_Camera.ImpactPoint` (`self.CameraRef`)) (`KismetMathLibrary.MakeVector` 0.0 (.y _worldlocation) (.z _worldlocation)) false false)
          (bind _returnvalue (`|CreateWidget` "/Game/Widget/WG_UIScale.WG_UIScale_C"))
          (bind _output_get (set `self.UIScaleRef` _returnvalue))
          (`UserWidget.AddToViewport` _output_get 0)
          ;;[1 1 1] Time dilatation
          (bind (_direction _timedilatation) (`Timeline|SetTimeDilatation` :!label _label)
            (:`Update`
              (`GameplayStatics.SetGlobalTimeDilation` (`KismetMathLibrary.Lerp` 1.0 (`self.MinDilatatonTime`) _timedilatation)))))
        (:`CastFailed`
          (set `self.b_HaveTarget` false)))))
  (:`Completed`
    (if (`self.b_HaveTarget`)
      (`Widget.RemoveFromParent` (`self.UIScaleRef`) :!label _label_2)
      (goto _label :!via `Reverse`))))

(event `StopScaling`
  ;[1 0 0] Scale system
  (if (`self.b_HaveTarget`)
    (set `self.b_HaveTarget` false)
    (goto _label_2)))

(fn `CalculateScale`
  (bind _worldlocation (`PlayerController.DeprojectMousePositionToWorld` (`GameplayStatics.GetPlayerController` 0)))
  (bind (_returnvalue_x _returnvalue_y _returnvalue_z) (`KismetMathLibrary.BreakVector` (`SceneComponent.K2_GetComponentLocation` (`/Game/Blueprints/Player/BP_Camera.ImpactPoint` (`self.CameraRef`)))))
  (bind _returnvalue (+ (`KismetMathLibrary.NormalizeToRange` (`KismetMathLibrary.Distance2D` (`KismetMathLibrary.MakeVector2D` _returnvalue_y _returnvalue_z) (`KismetMathLibrary.MakeVector2D` (.y _worldlocation) (.z _worldlocation))) 0.0 2.0) 1.0))
  (set `/Game/Widget/WG_UIScale.Lenght` _returnvalue (`self.UIScaleRef`))
  (`/Game/Blueprints/ScalablObject/BP_ScalableParent.Scale Object` (`self.TargetRef`) _returnvalue))

(fn `UserConstructionScript`)